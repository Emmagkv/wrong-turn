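; ScarySounds_BP is a wandering pawn that repeatedly emits an unsettling voice cue from its position.
; On BeginPlay, one loop uses AIMoveTo to reach random reachable points around its current location, pausing briefly after each success; a failed move ends the wandering.
; A parallel loop plays InsaneVoice_Cue at the pawn's location at random intervals of a few seconds.
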(event EventBeginPlay
  (Utilities|FlowControl|Sequence
    (:then_0
      (AI|AIMoveTo self (.RandomLocation (AI|Navigation|GetRandomReachablePointinRadius (Transformation|GetActorLocation) 1.5e+03 0 0)) 0 5.0 false :!label _label
        (:OnSuccess
          (Utilities|FlowControl|Delay 2.0)
          (goto _label))))
    (:then_1
      (Audio|PlaySoundatLocation "/Game/EK/Interact/sounds/InsaneVoice_Cue.InsaneVoice_Cue" (Transformation|GetActorLocation) "0, 0, 0" 1.0 1.0 0.0 0 0 0 0 :!label _label_2)
      (Utilities|FlowControl|Delay (Math|Conversions|ToFloat(Integer) (Math|Random|RandomIntegerinRange 3 6)))
      (goto _label_2))))

(fn ConstructionScript)