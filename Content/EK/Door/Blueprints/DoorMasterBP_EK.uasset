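; Master door Blueprint that swings open once enough tapes have been played.
; Each TapePlayed event increments a counter, and reaching TapesNeeded triggers OpenDoor once, playing a sound and rotating the door's yaw through a timeline.
; A box overlap toggles input and an interact prompt widget for the first-person character, but the Interact function is empty and no input events are handled here.
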(event OnComponentBeginOverlap(Box)
  (params (OverlappedComponent :type Primitive%20Component%20Object%20Reference) (OtherActor :type Actor%20Object%20Reference) (OtherComp :type Primitive%20Component%20Object%20Reference) (OtherBodyIndex :type Integer) (bFromSweep :type Boolean) (SweepResult :type Hit%20Result%20Structure%20%28by%20ref%29))
  ;[1 1 1] Enable input when near object
  (Utilities|Casting|CastToBP_FirstPersonCharacter OtherActor)
  (Input|EnableInput (Game|GetPlayerController 0))
  (bind _returnvalue (UserInterface|CreateWidget "/Game/EK/Interact/E_interactWidget.E_interactWidget_C" 0 (Variables|Default|GetText)))
  (UserInterface|Viewport|AddtoViewport _returnvalue 0))

(event OnComponentEndOverlap(Box)
  (params (OverlappedComponent :type Primitive%20Component%20Object%20Reference) (OtherActor :type Actor%20Object%20Reference) (OtherComp :type Primitive%20Component%20Object%20Reference) (OtherBodyIndex :type Integer))
  ;[1 1 1] Enable input when near object
  (Utilities|Casting|CastToBP_FirstPersonCharacter OtherActor)
  (Input|DisableInput (Game|GetPlayerController 0))
  (Widget|RemovefromParent (stale OnComponentBeginOverlap(Box) _returnvalue)))

(event Custom|OpenDoor
  ;[1 1 1] Door opening anim
  (Audio|PlaySoundatLocation "/Game/EK/Door/sounds/dooropen.dooropen" (Transformation|GetWorldLocation (Variables|Default|GetDoor)) "0, 0, 0" 1.0 1.0 0.0 0 0 0 0)
  (bind _door_rotation (Timeline|Open%20Door%20anim Play)
    (:Update
      (Transformation|SetRelativeRotation (Variables|Default|GetDoor) (Math|Rotator|MakeRotator 0.0 0.0 (Math|Float|Lerp 0.0 1.2e+02 _door_rotation)) false false))))

(event Custom|TapePlayed
  ;[1 1 1] Door opening conditions
  (bind _result (Math|Integer|IncrementInt (Variables|Default|GetTapesPlayed))
    (:%20%20
      (if (>= _result (Variables|Default|GetTapesNeeded))
        (Utilities|FlowControl|DoOnce false
          (:Completed
            (CallFunction|OpenDoor)))))))

(fn ConstructionScript)

(fn Interact
  (return))