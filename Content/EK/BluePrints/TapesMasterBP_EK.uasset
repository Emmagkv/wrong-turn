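; TapesMasterBP_EK is a base Blueprint for collectible audio tape pickups in the world.
; On Interact it plays a collect cue at the tape's location, then flags the first-person character as holding a tape and passes it this tape's audio reference before destroying itself.
; The AddToInventory function is an empty stub; pickup state lives directly on the character.
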(event EventInteract
  ;[1 1 1] Tape pickup and add to inventory
  (Audio|PlaySoundatLocation "/Game/EK/sounds/tapecollectcue.tapecollectcue" (Transformation|GetWorldLocation (Variables|Default|GetTape)) "0, 0, 0" 1.0 1.0 0.0 0 0 0 0)
  (bind _asbp_first_person_character (Utilities|Casting|CastToBP_FirstPersonCharacter (Game|GetPlayerCharacter 0)))
  (Variables|/Game/FirstPerson/Blueprints/BP_FirstPersonCharacter.BP_FirstPersonCharacter_C|SetHasTape _asbp_first_person_character true)
  (Variables|/Game/FirstPerson/Blueprints/BP_FirstPersonCharacter.BP_FirstPersonCharacter_C|Settaperef _asbp_first_person_character (Variables|Default|GetTapeAudio))
  (Actor|DestroyActor))

(fn ConstructionScript)

(fn AddtoInventory
  (return ""))