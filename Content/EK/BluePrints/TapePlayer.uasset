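; Interactable tape player that inserts and plays the tape the first-person character is holding, once only.
; Interact checks HasTape, shows the tape mesh, then runs timeline-driven PutInTape and CloseTop to slide it in and rotate the spring-arm lid shut, with sound cues.
; After a delay it plays the character's Taperef sound at Bottom's relative location.
; Tick stores the first TapesMasterBP_EK actor every frame, though Interact never reads it.
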(event EventTick
  (params (DeltaSeconds :type Float%20%28single-precision%29))
  ;[1 1 1] recognize the tapes
  (bind _outactors (Actor|GetAllActorsOfClass "/Game/EK/BluePrints/TapesMasterBP_EK.TapesMasterBP_EK_C"))
  (Variables|Default|SetTapeRef (Utilities|Array|Get(acopy) _outactors)))

(event EventInteract
  (bind _asbp_first_person_character (Utilities|Casting|CastToBP_FirstPersonCharacter (Game|GetPlayerCharacter 0)))
  ;[1 1 1] use player, insert and play tape
  (if (Variables|/Game/FirstPerson/Blueprints/BP_FirstPersonCharacter.BP_FirstPersonCharacter_C|GetHasTape _asbp_first_person_character)
    (Utilities|FlowControl|DoOnce false
      (:Completed
        (Rendering|SetVisibility (Variables|Default|GetTape) true false)
        (|PutInTape)
        (Utilities|FlowControl|Delay 1.0)
        (|CloseTop
          (:Get%20tape%20in
            (Utilities|FlowControl|Delay 3.5)
            (Audio|PlaySoundatLocation (Variables|/Game/FirstPerson/Blueprints/BP_FirstPersonCharacter.BP_FirstPersonCharacter_C|Gettaperef _asbp_first_person_character) (Variables|/Script/Engine.SceneComponent|GetRelativeLocation (Variables|Default|Getbottom)) "0, 0, 0" 1.0 1.0 0.0 0 0 0 0)))))))

(fn ConstructionScript)