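; DoorMasterBP_EK is a door Blueprint that swings open in response to tape collection.
; TapeCollect increments TapesCollected and, while that count is at most TapesNeeded, calls OpenDoor through a DoOnce, so the first qualifying pickup triggers it.
; OpenDoor plays a timeline that lerps the door's relative yaw from closed to 120 degrees.
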(event Custom|OpenDoor
  ;[1 1 1] Door opening anim
  (bind _door_rotation (Timeline|Open%20Door%20anim Play)
    (:Update
      (Transformation|SetRelativeRotation (Variables|Default|GetDoor) (Math|Rotator|MakeRotator 0.0 0.0 (Math|Float|Lerp 0.0 1.2e+02 _door_rotation)) false false))))

(event Custom|TapeCollect
  ;[1 1 1] Door opening conditions
  (Math|Integer|IncrementInt (Variables|Default|GetTapesCollected)
    (:%20%20
      (if (>= (Variables|Default|GetTapesNeeded) (Variables|Default|GetTapesCollected))
        (Utilities|FlowControl|DoOnce false
          (:Completed
            (CallFunction|OpenDoor)))))))

(fn ConstructionScript)