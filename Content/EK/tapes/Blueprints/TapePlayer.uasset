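; Interactable tape player that accepts a tape carried by the first-person character and plays its sound.
; A box overlap toggles player input and an interact widget.
; Interact runs once if the character has a tape, chaining timeline-driven tape insertion and lid closing with sound cues, then delayed playback of the character's tape sound.
; Tick also caches the first TapesMasterBP_EK actor every frame, though playback never uses it.
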(event OnComponentBeginOverlap(Box)
  (params (OverlappedComponent :type Primitive%20Component%20Object%20Reference) (OtherActor :type Actor%20Object%20Reference) (OtherComp :type Primitive%20Component%20Object%20Reference) (OtherBodyIndex :type Integer) (bFromSweep :type Boolean) (SweepResult :type Hit%20Result%20Structure%20%28by%20ref%29))
  ;[1 1 1] Enable input when near object
  (Utilities|Casting|CastToBP_FirstPersonCharacter OtherActor)
  (Input|EnableInput (Game|GetPlayerController 0))
  (bind _returnvalue (UserInterface|CreateWidget "/Game/EK/Interact/E_interactWidget.E_interactWidget_C" 0 (Variables|Default|GetText)))
  (UserInterface|Viewport|AddtoViewport _returnvalue 0))

(event OnComponentEndOverlap(Box)
  (params (OverlappedComponent :type Primitive%20Component%20Object%20Reference) (OtherActor :type Actor%20Object%20Reference) (OtherComp :type Primitive%20Component%20Object%20Reference) (OtherBodyIndex :type Integer))
  ;[1 1 1] Enable input when near object
  (Utilities|Casting|CastToBP_FirstPersonCharacter OtherActor)
  (Input|DisableInput (Game|GetPlayerController 0))
  (Widget|RemovefromParent (stale OnComponentBeginOverlap(Box) _returnvalue)))

(event EventTick
  (params (DeltaSeconds :type Float%20%28single-precision%29))
  ;[1 1 1] recognize the tapes
  (bind _outactors (Actor|GetAllActorsOfClass "/Game/EK/tapes/Blueprints/TapesMasterBP_EK.TapesMasterBP_EK_C"))
  (Variables|Default|SetTapeRef (Utilities|Array|Get(acopy) _outactors)))

(event EventInteract
  ;[1 1 1] use player, insert and play tape
  (bind _asbp_first_person_character (Utilities|Casting|CastToBP_FirstPersonCharacter (Game|GetPlayerCharacter 0)))
  (if (Variables|/Game/FirstPerson/Blueprints/BP_FirstPersonCharacter.BP_FirstPersonCharacter_C|GetHasTape _asbp_first_person_character)
    (Utilities|FlowControl|DoOnce false
      (:Completed
        (Rendering|SetVisibility (Variables|Default|GetTape) true false)
        (|PutInTape)
        (Utilities|FlowControl|Delay 1.0)
        (|CloseTop
          (:Get%20tape%20in
            (Utilities|FlowControl|Delay 3.5)
            (Audio|PlaySoundatLocation (Variables|/Game/FirstPerson/Blueprints/BP_FirstPersonCharacter.BP_FirstPersonCharacter_C|Gettaperef _asbp_first_person_character) (Variables|/Script/Engine.SceneComponent|GetRelativeLocation (Variables|Default|Getbottom)) "0, 0, 0" 1.0 1.0 0.0 0 0 0 0)))))))

(fn ConstructionScript)