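; Walkman pickup actor that the first-person player collects through its Interact event.
; Interacting sets HasWalkman on the character, plays a pickup sound and destroys the actor.
; Its box overlap enables input and shows an interact prompt widget, removed after a one-second delay or on exit, which also disables input.
; AddToInventory is a stub returning an empty value, and the construction script is empty.
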(event OnComponentBeginOverlap(Box)
  (params (OverlappedComponent :type Primitive%20Component%20Object%20Reference) (OtherActor :type Actor%20Object%20Reference) (OtherComp :type Primitive%20Component%20Object%20Reference) (OtherBodyIndex :type Integer) (bFromSweep :type Boolean) (SweepResult :type Hit%20Result%20Structure%20%28by%20ref%29))
  ;[1 1 1] Enable input when near object
  (Utilities|Casting|CastToBP_FirstPersonCharacter OtherActor)
  (Input|EnableInput (Game|GetPlayerController 0))
  (bind _returnvalue (UserInterface|CreateWidget "/Game/EK/Interact/E_interactWidget.E_interactWidget_C" 0 (Utilities|String|ToString(Text) (Variables|Default|GetText))))
  (UserInterface|Viewport|AddtoViewport _returnvalue 0)
  (Utilities|FlowControl|Delay 1.0)
  (Widget|RemovefromParent _returnvalue))

(event OnComponentEndOverlap(Box)
  (params (OverlappedComponent :type Primitive%20Component%20Object%20Reference) (OtherActor :type Actor%20Object%20Reference) (OtherComp :type Primitive%20Component%20Object%20Reference) (OtherBodyIndex :type Integer))
  ;[1 1 1] Enable input when near object
  (Utilities|Casting|CastToBP_FirstPersonCharacter OtherActor)
  (Input|DisableInput (Game|GetPlayerController 0))
  (Widget|RemovefromParent (stale OnComponentBeginOverlap(Box) _returnvalue)))

(event EventInteract
  ;[1 1 1] Pickup
  (bind _asbp_first_person_character (Utilities|Casting|CastToBP_FirstPersonCharacter (Game|GetPlayerCharacter 0)))
  (Variables|/Game/FirstPerson/Blueprints/BP_FirstPersonCharacter.BP_FirstPersonCharacter_C|SetHasWalkman? _asbp_first_person_character true)
  (Variables|Default|SetCharacterRef _asbp_first_person_character)
  (Audio|PlaySoundatLocation "/Game/EK/tapes/SoundCues/PickUp_Cue.PickUp_Cue" (Transformation|GetActorLocation _asbp_first_person_character) "0, 0, 0" 1.0 1.0 0.0 0 0 0 0)
  (Actor|DestroyActor))

(fn ConstructionScript)

(fn AddtoInventory
  (return ""))