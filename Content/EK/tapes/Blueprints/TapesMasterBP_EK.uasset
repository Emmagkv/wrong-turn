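; Master Blueprint for a collectible audio tape that, once played on the player's Walkman, notifies doors.
; Trigger overlap shows a timed prompt and toggles input; a separate event reveals the tape and enables collision.
; Interact requires HasWalkman, otherwise showing a hint; it hides the tape, sets HasTape and chains sounds with Delays timed to the clip.
; It then calls TapePlayed on the referenced Door and a class-found DoorMasterBP_EK, and destroys itself.
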(event OnComponentBeginOverlap(trigger)
  (params (OverlappedComponent :type Primitive%20Component%20Object%20Reference) (OtherActor :type Actor%20Object%20Reference) (OtherComp :type Primitive%20Component%20Object%20Reference) (OtherBodyIndex :type Integer) (bFromSweep :type Boolean) (SweepResult :type Hit%20Result%20Structure%20%28by%20ref%29))
  ;[1 1 1] Enable input when near object
  (Utilities|Casting|CastToBP_FirstPersonCharacter OtherActor)
  (Input|EnableInput (Game|GetPlayerController 0))
  (bind _returnvalue (UserInterface|CreateWidget "/Game/EK/Interact/E_interactWidget.E_interactWidget_C" 0 (Variables|Default|GetText)))
  (UserInterface|Viewport|AddtoViewport _returnvalue 0)
  (Utilities|FlowControl|Delay 1.0)
  (Widget|RemovefromParent _returnvalue))

(event OnComponentEndOverlap(trigger)
  (params (OverlappedComponent :type Primitive%20Component%20Object%20Reference) (OtherActor :type Actor%20Object%20Reference) (OtherComp :type Primitive%20Component%20Object%20Reference) (OtherBodyIndex :type Integer))
  ;[1 1 1] Enable input when near object
  (Utilities|Casting|CastToBP_FirstPersonCharacter OtherActor)
  (Input|DisableInput (Game|GetPlayerController 0))
  (Widget|RemovefromParent (stale OnComponentBeginOverlap(trigger) _returnvalue)))

(event Custom|SetVisibilityandinteraction
  (Rendering|SetVisibility (Variables|Default|GetTape) true false)
  (Rendering|SetVisibility (Variables|Default|Gettrigger) true false)
  (Collision|SetCollisionEnabled (Variables|Default|Gettrigger) "QueryAndPhysics"))

(event EventInteract
  (bind _tapeaudio (Variables|Default|GetTapeAudio))
  ;[1 1 1] Tape pickup and add to inventory
  (bind _asbp_first_person_character (Utilities|Casting|CastToBP_FirstPersonCharacter (Game|GetPlayerCharacter 0)))
  (if (Variables|/Game/FirstPerson/Blueprints/BP_FirstPersonCharacter.BP_FirstPersonCharacter_C|GetHasWalkman? _asbp_first_person_character)
    (Development|SetHiddeninGame (Variables|Default|GetTape) true true)
    (Variables|/Game/FirstPerson/Blueprints/BP_FirstPersonCharacter.BP_FirstPersonCharacter_C|SetHasTape _asbp_first_person_character true)
    (Variables|Default|SetcharaterRef _asbp_first_person_character)
    (bind _returnvalue (Actor|GetActorOfClass "/Game/FirstPerson/Blueprints/BP_FirstPersonCharacter.BP_FirstPersonCharacter_C"))
    (Audio|PlaySoundatLocation "/Game/EK/tapes/SoundCues/tapecollectcue.tapecollectcue" (Transformation|GetActorLocation _returnvalue) "0, 0, 0" 1.0 1.0 0.0 0 0 0 0)
    (Utilities|FlowControl|Delay 0.2)
    (Audio|PlaySoundatLocation "/Game/EK/tapes/SoundCues/tapeinsertcue.tapeinsertcue" (Transformation|GetActorLocation _returnvalue) "0, 0, 0" 1.0 1.0 0.0 0 0 0 0)
    (Utilities|FlowControl|Delay 1.2)
    (Audio|PlaySoundatLocation _tapeaudio (Transformation|GetActorLocation _returnvalue) "0, 0, 0" 1.0 1.0 0.0 0 0 0 0)
    (Utilities|FlowControl|Delay (Variables|/Script/Engine.SoundBase|GetDuration _tapeaudio))
    (Audio|PlaySoundatLocation "/Game/EK/tapes/SoundCues/closetopcue.closetopcue" (Transformation|GetActorLocation _returnvalue) "0, 0, 0" 1.0 1.0 0.0 0 0 0 0)
    (Utilities|FlowControl|Delay 0.5)
    (Audio|PlaySoundatLocation "/Game/EK/tapes/SoundCues/tapeinsertcue.tapeinsertcue" (Transformation|GetActorLocation _returnvalue) "0, 0, 0" 1.0 1.0 0.0 0 0 0 0)
    (Utilities|FlowControl|Delay 1.2)
    (bind _returnvalue_2 (Actor|GetActorOfClass "/Game/EK/Door/Blueprints/DoorMasterBP_EK.DoorMasterBP_EK_C"))
    (Default|TapePlayed _returnvalue_2)
    (Actor|DestroyActor)
    (else
      (bind _returnvalue_3 (UserInterface|CreateWidget "/Game/EK/Interact/E_interactWidget.E_interactWidget_C" 0 "I need something to play the tape!!!"))
      (UserInterface|Viewport|AddtoViewport _returnvalue_3 0)
      (Utilities|FlowControl|Delay 1.0)
      (Widget|RemovefromParent _returnvalue_3))))

(fn ConstructionScript)

(fn AddtoInventory
  (return ""))