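; BP_CutsceneTrigger is a box trigger that plays a one-time media cutscene when the first-person character walks in.
; On overlap it blocks look and move input, and a timeline lerps the first-person camera's relative rotation to a fixed angle.
; The timeline's update also chains fixed delays around opening the painting video on a media player, then sets the played flag and restores input.
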(event OnComponentBeginOverlap(Box)
  (params (OverlappedComponent :type Primitive%20Component%20Object%20Reference) (OtherActor :type Actor%20Object%20Reference) (OtherComp :type Primitive%20Component%20Object%20Reference) (OtherBodyIndex :type Integer) (bFromSweep :type Boolean) (SweepResult :type Hit%20Result%20Structure%20%28by%20ref%29))
  (bind _returnvalue (Game|GetPlayerController 0))
  (if (not (Variables|Default|GetCutsceneplayed?))
    (bind _asbp_first_person_character (Utilities|Casting|CastToBP_FirstPersonCharacter OtherActor))
    (Input|SetIgnoreLookInput _returnvalue true)
    (Input|SetIgnoreMoveInput _returnvalue true)
    (bind _movecamera (Timeline|Move%20Camera PlayFromStart)
      (:Update
        (Transformation|SetRelativeRotation (Variables|/Game/FirstPerson/Blueprints/BP_FirstPersonCharacter.BP_FirstPersonCharacter_C|GetFirstPersonCamera _asbp_first_person_character) (Math|Rotator|Lerp(Rotator) "0, 0, 0" "5.000000,0.000000,0.000000" _movecamera) false false)
        (Utilities|FlowControl|Delay 2.0)
        (Media|MediaPlayer|OpenSource (Variables|Default|GetMediaPlayer) "/Game/MartaStuff/PaintingAnim/PaintingFileMediaSource.PaintingFileMediaSource")
        (Utilities|FlowControl|Delay 2e+01)
        (Variables|Default|SetCutsceneplayed? true)
        (Input|SetIgnoreLookInput _returnvalue false)
        (Input|SetIgnoreMoveInput _returnvalue false)))))

(fn ConstructionScript)