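; NoteMaster_EK is a readable note actor that shows its image in a full-screen or overlay widget when the player interacts with it.
; A box overlap with the first-person character enables input on the actor and shows an interact prompt, both removed on exit.
; Interact alternates through a FlipFlop: it opens the note, locks look and move input and hides the actor, then puts it down and restores them, with a paper sound each time.
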(event OnComponentBeginOverlap(Box)
  (params (OverlappedComponent :type Primitive%20Component%20Object%20Reference) (OtherActor :type Actor%20Object%20Reference) (OtherComp :type Primitive%20Component%20Object%20Reference) (OtherBodyIndex :type Integer) (bFromSweep :type Boolean) (SweepResult :type Hit%20Result%20Structure%20%28by%20ref%29))
  ;[1 1 1] Enable input when near object
  (Utilities|Casting|CastToBP_FirstPersonCharacter OtherActor)
  (Input|EnableInput (Game|GetPlayerController 0))
  (bind _returnvalue (UserInterface|CreateWidget "/Game/EK/Interact/E_interactWidget.E_interactWidget_C" 0 (Variables|Default|GetText)))
  (UserInterface|Viewport|AddtoViewport _returnvalue 0))

(event OnComponentEndOverlap(Box)
  (params (OverlappedComponent :type Primitive%20Component%20Object%20Reference) (OtherActor :type Actor%20Object%20Reference) (OtherComp :type Primitive%20Component%20Object%20Reference) (OtherBodyIndex :type Integer))
  ;[1 1 1] Enable input when near object
  (Utilities|Casting|CastToBP_FirstPersonCharacter OtherActor)
  (Input|DisableInput (Game|GetPlayerController 0))
  (Widget|RemovefromParent (stale OnComponentBeginOverlap(Box) _returnvalue)))

(event EventInteract
  (bind _returnvalue (Game|GetPlayerController 0))
  (bind _note (Variables|Default|Getnote))
  (bind _returnvalue_2 (Transformation|GetWorldLocation _note))
  ;[1 1 1] Interact and show Note widget
  (Utilities|FlowControl|FlipFlop
    (:A
      (Audio|PlaySoundatLocation "/Game/EK/Notes/Sounds/paperCollectQue.paperCollectQue" _returnvalue_2 "0, 0, 0" 1.0 1.0 0.0 0 0 0 0)
      (bind _returnvalue_3 (UserInterface|CreateWidget "/Game/EK/Notes/Widgets/Note_Widget.Note_Widget_C" 0 (Variables|Default|GetNoteRef)))
      (UserInterface|Viewport|AddtoViewport _returnvalue_3 0)
      (Input|SetIgnoreLookInput _returnvalue true)
      (Input|SetIgnoreMoveInput _returnvalue true)
      (Rendering|SetActorHiddenInGame true))
    (:B
      (Audio|PlaySoundatLocation "/Game/EK/Notes/Sounds/paperCollectQue.paperCollectQue" _returnvalue_2 "0, 0, 0" 1.0 1.0 0.0 0 0 0 0)
      (Default|PutDown _returnvalue_3)
      (Input|SetIgnoreLookInput _returnvalue false)
      (Input|SetIgnoreMoveInput _returnvalue false)
      (Rendering|SetActorHiddenInGame false))))

(fn ConstructionScript)