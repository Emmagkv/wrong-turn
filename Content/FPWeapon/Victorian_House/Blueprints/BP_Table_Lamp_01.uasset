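; Interactable table lamp Blueprint that switches its light on and off and highlights itself while focused.
; Interacting toggles the point light, flip-flops bulb emissive via new dynamic material instances, and plays a sound at world origin.
; Focus optionally enables a custom-depth outline and shows a widget once through DoN, while a retriggerable delay clears both when focus calls stop.
; Construction script sets initial light visibility from LightOnoff, leaving emissive untouched.
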(event Custom|ResetOff
  ;[1 1 1] Outline
  (Utilities|FlowControl|DoN 1) ; enters at Reset
)

(event EventOnInteract
  ;[1 1 1] on/off Light
  (Rendering|ToggleVisibility (Variables|Default|GetPointLight) false)
  (Utilities|FlowControl|FlipFlop
    (:A
      (bind _returnvalue (Rendering|Material|CreateDynamicMaterialInstance (Variables|Default|GetLamp) 1 "/Game/FPWeapon/Victorian_House/Materials/Instance/Tiling/Inst_Plastic_Glossy_01.Inst_Plastic_Glossy_01" "None" :!class /Script/Engine.PrimitiveComponent))
      (Variables|Default|SetDynamic%20material _returnvalue)
      (Rendering|Material|SetScalarParameterValue (Variables|Default|GetDynamic%20material) "PowerEmissive" 5.0 :!class /Script/Engine.MaterialInstanceDynamic))
    (:B
      (bind _returnvalue_2 (Rendering|Material|CreateDynamicMaterialInstance (Variables|Default|GetLamp) 1 "/Game/FPWeapon/Victorian_House/Materials/Instance/Tiling/Inst_Plastic_Glossy_01.Inst_Plastic_Glossy_01" "None" :!class /Script/Engine.PrimitiveComponent))
      (Variables|Default|SetDynamic%20material _returnvalue_2)
      (Rendering|Material|SetScalarParameterValue (Variables|Default|GetDynamic%20material) "PowerEmissive" 0.0 :!class /Script/Engine.MaterialInstanceDynamic)))
  (Audio|PlaySoundatLocation "/Game/FPWeapon/Victorian_House/Audio/Cues/Cue_Light.Cue_Light" "0, 0, 0" "0, 0, 0" 1.0 1.0 0.0 0 0 0 0))

(event EventOnFocus
  ;[1 1 1] Outline
  (Utilities|FlowControl|Sequence
    (:then_0
      (if (Variables|Default|GetOutline%20on/off)
        (CallFunction|BeginFocus))
      (Variables|Default|SetTimeOutlineEnd 0.1)
      (Utilities|FlowControl|RetriggerableDelay (Variables|Default|GetTimeOutlineEnd))
      (CallFunction|EndFocus)
      (Widget|RemovefromParent (stale _returnvalue))
      (CallFunction|ResetOff))
    (:then_1
      (Utilities|FlowControl|DoN 1
        (:Exit
          (bind _returnvalue (UserInterface|CreateWidget "/Game/FPWeapon/Victorian_House/UMG/LightOff_Widget.LightOff_Widget_C"))
          (UserInterface|Viewport|AddtoViewport _returnvalue 0))))))

(fn ConstructionScript
  ;[1 1 1] on/off Light
  (Rendering|SetVisibility (Variables|Default|GetPointLight) (Variables|Default|GetLight%20on/off%20) false))

(fn BeginFocus
  (Rendering|SetRenderCustomDepth (Variables|Default|GetLamp) true))

(fn EndFocus
  (Rendering|SetRenderCustomDepth (Variables|Default|GetLamp) false))